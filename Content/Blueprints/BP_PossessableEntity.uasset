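; BP_PossessableEntity is a possessable entity with a camera and spring arm that moves in a supplied direction.
; Its Move event feeds the vector into movement input, then snaps the capsule's world yaw to the camera's, zeroing pitch and roll.
; Two getters expose forward and right vectors, taken from the spring arm rather than the camera itself.
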(event `Move`
  (params (Vector :type "Vector Structure"))
  (bind (_returnvalue_roll _returnvalue_pitch _returnvalue_yaw) (`KismetMathLibrary.BreakRotator` (`SceneComponent.K2_GetComponentRotation` (`self.Camera`))))
  (`self.AddMovementInput` Vector)
  (`SceneComponent.K2_SetWorldRotation` (`self.CapsuleComponent`) (`KismetMathLibrary.MakeRotator` 0.0 0.0 _returnvalue_yaw) false false))

(fn `GetCameraForwardVector`
  (returns (NewParam :type "Vector Structure"))
  (return (`SceneComponent.GetForwardVector` (`self.SpringArm`))))

(fn `GetCameraRightVector`
  (returns (NewParam :type "Vector Structure"))
  (return (`SceneComponent.GetRightVector` (`self.SpringArm`))))

(fn `UserConstructionScript`)