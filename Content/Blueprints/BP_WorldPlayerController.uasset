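; BP_WorldPlayerController is the player controller that routes Enhanced Input movement and look to the possessed pawn.
; On BeginPlay it hides the cursor, sets Game and UI input mode with mouse lock on capture, and adds IMC_Player.
; IA_Move combines the pawn's horizontal forward and right vectors and passes the result to Move on BP_PossessableEntity.
; IA_Look feeds pitch and yaw input directly to the controller.
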(event `self.ReceiveBeginPlay`
  (set `self.bShowMouseCursor` false)
  (`WidgetBlueprintLibrary.SetInputMode_GameAndUIEx` self null "LockOnCapture")
  (`EnhancedInputSubsystemInterface.AddMappingContext` (subsystem `EnhancedInputLocalPlayerSubsystem`) "/Game/Assets/Input/IMC_Player.IMC_Player" 0 (struct)))

(event `EnhancedInput|/Game/Assets/Input/InputActions/IA_Move`
  (params (ActionValue :type "Vector2D Structure") (ElapsedSeconds :type "Float (double-precision)") (TriggeredSeconds :type "Float (double-precision)") (InputAction :type "InputAction Object Reference" :default "/Game/Assets/Input/InputActions/IA_Move.IA_Move"))
  (bind (_x _y) (`KismetMathLibrary.BreakVector2D` ActionValue))
  (bind _returnvalue (`self.K2_GetPawn`))
  (bind (_returnvalue_x _returnvalue_y) (`KismetMathLibrary.BreakVector` (`self.GetActorRightVector` _returnvalue)))
  (bind (_returnvalue_x_2 _returnvalue_y_2) (`KismetMathLibrary.BreakVector` (`self.GetActorForwardVector` _returnvalue)))
  (:`Triggered`
    (`/Game/Blueprints/BP_PossessableEntity.Move` (cast `/Game/Blueprints/BP_PossessableEntity` _returnvalue :!pure true) (+ (* _y (`KismetMathLibrary.MakeVector` _returnvalue_x_2 _returnvalue_y_2)) (* (`KismetMathLibrary.MakeVector` _returnvalue_x _returnvalue_y) _x)))))

(event `EnhancedInput|/Game/Assets/Input/InputActions/IA_Look`
  (params (ActionValue :type "Vector2D Structure") (ElapsedSeconds :type "Float (double-precision)") (TriggeredSeconds :type "Float (double-precision)") (InputAction :type "InputAction Object Reference" :default "/Game/Assets/Input/InputActions/IA_Look.IA_Look"))
  (bind (_x _y) (`KismetMathLibrary.BreakVector2D` ActionValue))
  (:`Triggered`
    (`self.AddPitchInput` _y)
    (`self.AddYawInput` _x)))

(fn `UserConstructionScript`)